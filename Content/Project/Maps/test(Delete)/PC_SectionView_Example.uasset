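; Example player controller that demonstrates switching a section view between preset height markers.
; On BeginPlay it finds the level's BP_SectionView actor, adds the example UI widget to the viewport and shows the mouse cursor.
; Number keys 1 to 5 derive an index from the pressed key's display name and pass the matching height marker to BP_SectionView to update the view.
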(event `self.ReceiveBeginPlay`
  (bind _returnvalue (`GameplayStatics.GetActorOfClass` "/Game/Project/Maps/Blueprints/BP_SectionView.BP_SectionView_C"))
  (set `self.BP_SectionView` _returnvalue)
  (bind _returnvalue_2 (`|CreateWidget` "/Game/Project/Maps/test(Delete)/UW_SectionView_Example.UW_SectionView_Example_C"))
  (bind _output_get (set `self.UW_main` _returnvalue_2))
  (`UserWidget.AddToViewport` _output_get 0)
  (set `self.bShowMouseCursor` true))

(event `Key|One`
  (params (Key :type "Key Structure"))
  (bind _bp_sectionview (`self.BP_SectionView`))
  (:`Pressed`
    (set `self.Key` (`self.GetKeyNumber` Key))
    (`/Game/Project/Maps/Blueprints/BP_SectionView.UpdateSectionViewUsingHeightMarker` _bp_sectionview (`|GetArrayItem` (`/Game/Project/Maps/Blueprints/BP_SectionView.HeightMarkers` _bp_sectionview) (- (`self.Key`) 1)) :!label _label)))

(event `Key|Two`
  (params (Key :type "Key Structure"))
  (:`Pressed`
    (set `self.Key` (`self.GetKeyNumber` Key))
    (goto _label)))

(event `Key|Three`
  (params (Key :type "Key Structure"))
  (:`Pressed`
    (set `self.Key` (`self.GetKeyNumber` Key))
    (goto _label)))

(event `Key|Four`
  (params (Key :type "Key Structure"))
  (:`Pressed`
    (set `self.Key` (`self.GetKeyNumber` Key))
    (goto _label)))

(event `Key|Five`
  (params (Key :type "Key Structure"))
  (:`Pressed`
    (set `self.Key` (`self.GetKeyNumber` Key))
    (goto _label)))

(fn `GetKeyNumber`
  (params (Key :type "Key Structure (by ref)"))
  (returns (ReturnValue :type Integer))
  (return (`KismetStringLibrary.Conv_StringToInt` (`KismetTextLibrary.Conv_TextToString` (`KismetInputLibrary.Key_GetDisplayName` Key)))))

(fn `UserConstructionScript`)
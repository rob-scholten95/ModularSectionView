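; BP_SectionView_HeightMarker is a section view height marker that can fade in and out with a holographic look.
; BeginPlay gives the Marker a dynamic M_Holo material, starting fully transparent in NormalColor, with SetMaterialColor setting its Color parameter.
; Fade restarts a Timeline that drives Opacity_Total from its current value toward VisibleOpacity or zero.
; The Timeline alpha feeds FInterpTo's DeltaTime at speed 1, so it effectively acts as a lerp.
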(event `self.ReceiveBeginPlay`
  (bind _returnvalue (`KismetMaterialLibrary.CreateDynamicMaterialInstance` "/Game/Project/Materials/Holo/M_Holo.M_Holo"))
  (bind _output_get (set `self.dynamic_mat` _returnvalue))
  (`PrimitiveComponent.SetMaterial` (`self.Marker`) 0 _output_get)
  (`MaterialInstanceDynamic.SetScalarParameterValue` _output_get "Opacity_Total" 0.0)
  (`self.SetMaterialColor` (`self.Normal Color`)))

(event `Fade`
  (params (`Fade In` :type Boolean))
  (bind _dynamic_mat (`self.dynamic_mat`))
  (bind _returnvalue (`MaterialInstanceDynamic.K2_GetScalarParameterValue` (`self.dynamic_mat`) "Opacity_Total"))
  (bind _output_get (set `self.CurrentOpacity` _returnvalue))
  (if `Fade In`
    (set `self.NewOpacity` (`self.VisibleOpacity`))
    (bind (_direction _alpha) (`Timeline|Timeline` :!via `PlayFromStart` :!label _label)
      (:`Update`
        (bind _output_get_2 (set `self.Interpolated` (`KismetMathLibrary.FInterpTo` (`self.CurrentOpacity`) (`self.NewOpacity`) _alpha 1.0)))
        (`MaterialInstanceDynamic.SetScalarParameterValue` _dynamic_mat "Opacity_Total" _output_get_2))
      (:`Finished`
        (bind _returnvalue_2 (`MaterialInstanceDynamic.K2_GetScalarParameterValue` _dynamic_mat "Opacity_Total"))
        (set `self.CurrentOpacity` _returnvalue_2)))
    (else
      (set `self.NewOpacity` 0.0)
      (goto _label :!via `PlayFromStart`))))

(event `self.ReceiveTick`
  (params (DeltaSeconds :type "Float (single-precision)")))

(fn `SetMaterialColor`
  (params (Value :type "LinearColor Structure"))
  (`MaterialInstanceDynamic.SetVectorParameterValue` (`self.dynamic_mat`) "Color" Value))

(fn `UserConstructionScript`)
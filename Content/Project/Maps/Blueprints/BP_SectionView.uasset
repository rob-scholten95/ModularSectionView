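; BP_SectionView drives a section-view cutaway by writing a box component's location, bounds and yaw into the SectionMask material parameter collection.
; Clicking a height marker, or passing a Z height, moves the box's bottom to that height; reclicking the selected marker resets it.
; A looping timer replaces Tick to interpolate the parameters, with a gate that closes once location and bounds converge.
; Markers change color and fade with hover, selection and mode.
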(event `self.ReceiveBeginPlay`
  (bind _sectionview (`self.SectionView`))
  (bind (_origin _boxextent) (`KismetSystemLibrary.GetComponentBounds` _sectionview))
  (bind (_returnvalue_roll _returnvalue_pitch _returnvalue_yaw) (`KismetMathLibrary.BreakRotator` (`SceneComponent.K2_GetComponentRotation` _sectionview)))
  ;[1 1 1] BEGINPLAY
  (`|ExecutionSequence`
    (:`then_0`
      ;;[1 1 1] Set the initial data for the box component so it can be used later to reset the section view
      (set `self.InitialSectionView` (make `/Game/Project/Maps/Utilities/S_InitialSectionView` _origin (* _boxextent 2.0) (/ (`KismetMathLibrary.ClampAxis` _returnvalue_yaw) 360.0))))
    (:`then_1`
      ;;[1 0.8261 0.1073] Enable the Custom Tick on BeginPlay (This can be done elsewhere if needed for performance reasons)
      (`self.EnableUpdateSectionViewTick` true))
    (:`then_2`
      ;;[1 1 1] Collect and store the height markers in the scene.
      (if (`self.UseHeightMarkers`)
        (bind _outactors (`GameplayStatics.GetAllActorsOfClass` "/Game/Project/Maps/Blueprints/BP_SectionView_HeightMarker.BP_SectionView_HeightMarker_C"))
        (if (`KismetArrayLibrary.Array_IsNotEmpty` _outactors)
          (set `self.HeightMarkers` _outactors)
          (else
            (`KismetSystemLibrary.PrintString` "No Height Markers detected in the scene!" true true (struct :`R` 1.0 :`G` 0.087192 :`A` 1.0) 15.0)))))
    (:`then_3`
      ;;[1 1 1] Set the section view volume to match the box location at BeginPlay
      (`self.SetSectionVolumeZ` (.z (`self.K2_GetActorLocation`))))
    (:`then_4`
      ;;[1 1 1] Comment
      (for _array_element (`self.HeightMarkers`)
        (add `self.OnBeginCursorOver` _array_element (`|CreateDelegate` :!event `OnBeginCursorOverMarker`))
        (add `self.OnEndCursorOver` _array_element (`|CreateDelegate` :!event `OnEndCursorOverMarker`))
        (add `self.OnClicked` _array_element (`|CreateDelegate` :!event `OnClickedMarker`))))))

(event `OnSelectedHeightMarkerChanged`)

(event `UpdateSectionView`
  (bind _sectionview (`self.SectionView`))
  (bind (_origin _boxextent) (`KismetSystemLibrary.GetComponentBounds` _sectionview))
  (bind (_returnvalue_roll _returnvalue_pitch _returnvalue_yaw) (`KismetMathLibrary.BreakRotator` (`SceneComponent.K2_GetComponentRotation` _sectionview)))
  ;[0.4757 1 1 1 100] SECTION VIEW
  ;;[1 1 1] Main Section view logic
  (`self.SectionViewMask` (`KismetMathLibrary.Conv_VectorToLinearColor` _origin) (`KismetMathLibrary.Conv_VectorToLinearColor` (* _boxextent 2.0)) (/ (`KismetMathLibrary.ClampAxis` _returnvalue_yaw) 360.0) :!label _label))

(event `OpenUpdateSectionView`
  ;[0.4757 1 1 1 100] SECTION VIEW
  ;;[1 1 1] Main Section view logic
  (`self.IsSectionViewModeEnabled`)
  (goto _label :!via `Open`))

(event `SetSectionVolumeZ`
  (params (`New Z` :type "Float (double-precision)"))
  (bind _sectionview (`self.SectionView`))
  (bind (_returnvalue_x _returnvalue_y) (`KismetMathLibrary.BreakVector` (`SceneComponent.K2_GetComponentLocation` _sectionview)))
  ;[0.4757 1 1 1 100] SECTION VIEW
  ;;[1 1 1] Set New height for the box component and then update section view
  (`self.IsSectionViewModeEnabled`)
  (`SceneComponent.K2_SetWorldLocation` (`self.SectionView`) (`KismetMathLibrary.MakeVector` _returnvalue_x _returnvalue_y (+ `New Z` (.z (`.BoxExtent` (`KismetSystemLibrary.GetComponentBounds` _sectionview))))) false false)
  (`self.OpenUpdateSectionView`))

(event `EnableUpdateSectionViewTick`
  (params (Enabled :type Boolean))
  ;[0.4757 1 1 1 100] SECTION VIEW
  ;;[1 1 1] Enable the Tick necessary for this blueprint to function, can be turned on or off for performance reasons and time can be determined
  (if Enabled
    (if (`KismetSystemLibrary.K2_IsValidTimerHandle` (`self.Timer`))
      (`KismetSystemLibrary.PrintString` "EnableUpdateSectionnViewTick is already enabled!")
      (else
        (bind _returnvalue (`KismetSystemLibrary.K2_SetTimerDelegate` (`|CreateDelegate` :!event `UpdateSectionView`) (`self.CustomTickTime`) true))
        (set `self.Timer` _returnvalue)))
    (elif (`KismetSystemLibrary.K2_IsValidTimerHandle` (`self.Timer`))
      (`KismetSystemLibrary.K2_ClearAndInvalidateTimerHandle` (`self.Timer`))
      (else
        (`KismetSystemLibrary.PrintString` "EnableUpdateSectionnViewTick is already disabled!")))))

(event `ResetSectionView`
  (bind _initialsectionview_location (break `/Game/Project/Maps/Utilities/S_InitialSectionView` (`self.InitialSectionView`)))
  ;[0.4757 1 1 1 100] SECTION VIEW
  ;;[0.5409 1 0.5443 1 35] Public Functions
  ;;;[1 1 1] Reset the section view to its original position at the start of the beginplay
  (`self.SetSectionVolumeZ` (.z _initialsectionview_location)))

(event `UpdateSectionViewUsingHeightMarker`
  (params (`Height Marker` :type "/Game/Project/Maps/Blueprints/BP_SectionView_HeightMarker Object Reference"))
  ;[0.4757 1 1 1 100] SECTION VIEW
  ;;[0.5409 1 0.5443 1 35] Public Functions
  ;;;[1 1 1] Update section using the height marker objects. Make sure the boolean is enabled and there are height markers in the scene!
  (`self.SetSectionVolumeZ` (.z (`self.K2_GetActorLocation` `Height Marker`))))

(event `UpdateSectionViewUsingZHeight`
  (params (`New Z` :type "Float (double-precision)"))
  ;[0.4757 1 1 1 100] SECTION VIEW
  ;;[0.5409 1 0.5443 1 35] Public Functions
  ;;;[1 1 1] Update section using the input of Z height coming externally
  (`self.SetSectionVolumeZ` `New Z`))

(event `EnableSectionViewMode`
  (params (Enabled :type Boolean))
  ;[0.4757 1 1 1 100] SECTION VIEW
  ;;[0.5409 1 0.5443 1 35] Public Functions
  ;;;[1 1 1] Enable Section View Mode
  (`self.EnableUpdateSectionViewTick` Enabled)
  (bind _output_get (set `self.SectionViewModeEnabled` Enabled))
  (`self.FadeAllHeightMarkers` _output_get))

(fn `FadeAllHeightMarkers`
  (params (Enabled :type Boolean))
  (for _array_element (`self.HeightMarkers`)
    (`/Game/Project/Maps/Blueprints/BP_SectionView_HeightMarker.Fade` _array_element Enabled)))

(fn `OnBeginCursorOverMarker`
  (params (TouchedActor :type "Actor Object Reference"))
  (bind _asbp_section_view_height_marker (cast `/Game/Project/Maps/Blueprints/BP_SectionView_HeightMarker` TouchedActor))
  (bind _output_get (set `self.HoveredActor` _asbp_section_view_height_marker))
  (`/Game/Project/Maps/Blueprints/BP_SectionView_HeightMarker.SetMaterialColor` _output_get (`self.Hovered Color`)))

(fn `OnClickedMarker`
  (params (TouchedActor :type "Actor Object Reference") (ButtonPressed :type "Key Structure" :default "None"))
  (bind _selectedactor (`self.SelectedActor`))
  (bind _asbp_section_view_height_marker (cast `/Game/Project/Maps/Blueprints/BP_SectionView_HeightMarker` TouchedActor))
  (`/Engine/EditorBlueprintResources/StandardMacros.IsValid` _selectedactor
    (:`Is Valid`
      (if (== _selectedactor _asbp_section_view_height_marker)
        (for _array_element (`self.HeightMarkers`)
          (`/Game/Project/Maps/Blueprints/BP_SectionView_HeightMarker.Fade` _array_element true))
        (`/Game/Project/Maps/Blueprints/BP_SectionView_HeightMarker.SetMaterialColor` (`self.SelectedActor`) (`self.Normal Color`))
        (set `self.SelectedActor` null)
        (`self.ResetSectionView`)
        (else
          (for _array_element_2 (`self.HeightMarkers`)
            (`/Game/Project/Maps/Blueprints/BP_SectionView_HeightMarker.Fade` _array_element_2 true))
          (`/Game/Project/Maps/Blueprints/BP_SectionView_HeightMarker.SetMaterialColor` (`self.SelectedActor`) (`self.Normal Color`))
          (bind _output_get (set `self.SelectedActor` _asbp_section_view_height_marker))
          (`/Game/Project/Maps/Blueprints/BP_SectionView_HeightMarker.SetMaterialColor` _output_get (`self.Selected Color`))
          (`self.UpdateSectionViewUsingHeightMarker` (`self.SelectedActor`) :!label _label))))
    (:`Is Not Valid`
      (bind _output_get_2 (set `self.SelectedActor` _asbp_section_view_height_marker))
      (`/Game/Project/Maps/Blueprints/BP_SectionView_HeightMarker.SetMaterialColor` _output_get_2 (`self.Selected Color`))
      (for _array_element_3 (`self.HeightMarkers`)
        (if (not (== _array_element_3 (`self.SelectedActor`)))
          (`/Game/Project/Maps/Blueprints/BP_SectionView_HeightMarker.Fade` _array_element_3 false)))
      (goto _label))))

(fn `OnEndCursorOverMarker`
  (params (TouchedActor :type "Actor Object Reference"))
  (bind _asbp_section_view_height_marker (cast `/Game/Project/Maps/Blueprints/BP_SectionView_HeightMarker` TouchedActor))
  (if (not (== _asbp_section_view_height_marker (`self.SelectedActor`)))
    (bind _asbp_section_view_height_marker_2 (cast `/Game/Project/Maps/Blueprints/BP_SectionView_HeightMarker` TouchedActor))
    (`/Game/Project/Maps/Blueprints/BP_SectionView_HeightMarker.SetMaterialColor` _asbp_section_view_height_marker_2 (`self.Normal Color`))
    (set `self.HoveredActor` null)))

(fn `UserConstructionScript`)